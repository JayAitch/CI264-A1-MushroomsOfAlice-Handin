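; Lockable hinged door Blueprint that swings open and closed when OpenDoor is called while unlocked.
; A timeline drives the door's yaw up to OpenAngle, reverses to close, and flips IsDoorOpen on finish.
; BeginPlay initializes the timeline and applies the starting material through MaterialChanger.
; DoorLockUnlock toggles the lock state and passes it to MaterialChanger to update the door's material.
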(event `self.ReceiveBeginPlay`
  ;[1 1 1] init door method
  ;;[0.4993 1 0.45] already open?
  (`self.SetTimeOfDoor` (`self.IsDoorOpen`))
  (`/Game/MyAssets/Components/MaterialChanger.Change Material` (`self.MaterialChanger`) (`self.Door`) (`self.StartMaterialInt`)))

(event `OpenDoor`
  (bind _isdooropen (`self.IsDoorOpen`))
  ;[1 1 1] Door opening/closing
  (if (`self.UnlockedDoor`)
    (if (not (`self.IsDoorOpen`))
      (if (not _isdooropen)
        (bind (_direction _doorrotator) (`Timeline|DoorTimeline` :`NewTime` (`KismetMathLibrary.SelectFloat` (`TimelineComponent.GetTimelineLength` (`self.DoorTimeline`)) 0.0 (stale `SetTimeOfDoor` IsDoorOpen)) :!label _label)
          (:`Update`
            ;;[0.6417 0.5249 1] Act on door rotation
            (`SceneComponent.K2_SetRelativeRotation` (`self.Door`) (`KismetMathLibrary.MakeRotator` 0.0 0.0 (* _doorrotator (`self.OpenAngle`))) false false))
          (:`Finished`
            ;;;[1 0.3397 0.4095] Switch open bool after opening/closing
            (set `self.IsDoorOpen` (not (`self.IsDoorOpen`))))))
      (elif _isdooropen
        (goto _label :!via `Reverse`)))))

(event `SetTimeOfDoor`
  (params (IsDoorOpen :type Boolean))
  ;[1 1 1] Door opening/closing
  ;;[0.966 0.562 1] Set Door Timeline based on door closed/open
  (goto _label :!via `SetNewTime`))

(event `DoorLockUnlock`
  ;[1 1 1] Change door material on door unlock and set door unlock bool
  (bind _output_get (set `self.UnlockedDoor` (not (`self.UnlockedDoor`))))
  (`/Game/MyAssets/Components/MaterialChanger.LockingUnlocking` (`self.MaterialChanger`) _output_get))

(fn `UserConstructionScript`)